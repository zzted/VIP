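; Interactable map prop that rolls and unrolls when the player interacts with it, extending a parent class's interaction logic.
; Each interaction toggles a flag and plays or reverses the UnrollMap timeline, which scrubs the skeletal mesh's animation position from its rolled starting pose.
; Two query-only boxes swap on each toggle so collision matches the extended or unextended state.
; Highlight events toggle custom depth rendering on the mesh.
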(event `self.ReceiveBeginPlay`
  (`parent.ReceiveBeginPlay`)
  (`SkeletalMeshComponent.SetPosition` (`self.SkeletalMesh`) 1.0 true)
  (`self.UnextendCollision`))

(event `/Game/BP/BPI_Interactable.OnInteract`
  (`|ExecutionSequence`
    (:`then_0`
      (`parent.OnInteract`))
    (:`then_1`
      (if (`self.Unrolling`)
        (`self.UnextendCollision`)
        (set `self.Unrolling` false)
        (bind (_direction _alpha) (`Timeline|UnrollMap` :!via `Reverse` :!label _label)
          (:`Update`
            (`SkeletalMeshComponent.SetPosition` (`self.SkeletalMesh`) (`KismetMathLibrary.Lerp` 1.0 0.0 _alpha) false)))
        (else
          (`self.ExtendCollision`)
          (set `self.Unrolling` true)
          (goto _label))))))

(event `/Game/BP/BPI_Highlightable.Highlight`
  (`PrimitiveComponent.SetRenderCustomDepth` (`self.SkeletalMesh`) true))

(event `/Game/BP/BPI_Highlightable.UnHighlight`
  (`PrimitiveComponent.SetRenderCustomDepth` (`self.SkeletalMesh`) false))

(fn `ExtendCollision`
  (`PrimitiveComponent.SetCollisionEnabled` (`self.Box_Extended`) "QueryOnly")
  (`PrimitiveComponent.SetCollisionEnabled` (`self.Box_Unextended`) "NoCollision"))

(fn `UnextendCollision`
  (`PrimitiveComponent.SetCollisionEnabled` (`self.Box_Extended`) "NoCollision")
  (`PrimitiveComponent.SetCollisionEnabled` (`self.Box_Unextended`) "QueryOnly"))

(fn `UserConstructionScript`)