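; Inspectable crystal ball puzzle: the player drags to rotate it until a scattered Niagara point cloud resolves into a hidden image.
; BeginPlay scatters data table cat points in random depth within the sphere, scaling X/Y by perspective so they align from one view.
; While inspecting, Tick maps up-vector alignment with camera forward to particle locomotion strength.
; Holding alignment past a timer marks it solved; breaking alignment resets it.
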(event EventHighlight
  (Development|PrintString "Highlight")
  (Rendering|SetRenderCustomDepth (Variables|Default|GetSphere) true))

(event EventUnHighlight
  (Development|PrintString "UnHighlight")
  (Rendering|SetRenderCustomDepth (Variables|Default|GetSphere) false))

(event EventOnInteract
  (|CallParentFunction))

(event EventBeginPlay
  (bind _cameradistanceoffsetstrength (Variables|Default|GetCameraDistanceOffsetStrength))
  (bind _cameradistance (Variables|Default|GetCameraDistance))
  (bind _returnvalue (* _cameradistance _cameradistanceoffsetstrength))
  (|CallParentFunction)
  (bind _outrownames (DataTable|GetDataTableRowNames (Variables|Default|GetCatTable)))
  (for _array_element _outrownames
    (bind _returnvalue_2 (Utilities|GetDataTableRow "/Game/BP/CrystalBall/DT_CatPoints.DT_CatPoints" _array_element)
      (:then
        (Utilities|Array|Add (Variables|Default|GetPointCloud) (Math|Vector|MakeVector (* (* (* (.x _returnvalue_2) (Variables|Default|GetSphereRadius)) (Variables|Default|GetAspectRatio)) (/ (- _returnvalue (Math|Random|RandomFloatinRange (* (|(sqrt((((square(R))-(square((X*R))))-(square((Y*R)))))) (Variables|Default|GetSphereRadius) (.x _returnvalue_2) (.y _returnvalue_2)) -1.0) (|(sqrt((((square(R))-(square((X*R))))-(square((Y*R)))))) (Variables|Default|GetSphereRadius) (.x _returnvalue_2) (.y _returnvalue_2)))) _returnvalue)) (* (* (.y _returnvalue_2) (Variables|Default|GetSphereRadius)) (/ (- _returnvalue (Math|Random|RandomFloatinRange (* (|(sqrt((((square(R))-(square((X*R))))-(square((Y*R)))))) (Variables|Default|GetSphereRadius) (.x _returnvalue_2) (.y _returnvalue_2)) -1.0) (|(sqrt((((square(R))-(square((X*R))))-(square((Y*R)))))) (Variables|Default|GetSphereRadius) (.x _returnvalue_2) (.y _returnvalue_2)))) _returnvalue)) (Math|Random|RandomFloatinRange (* (|(sqrt((((square(R))-(square((X*R))))-(square((Y*R)))))) (Variables|Default|GetSphereRadius) (.x _returnvalue_2) (.y _returnvalue_2)) -1.0) (|(sqrt((((square(R))-(square((X*R))))-(square((Y*R)))))) (Variables|Default|GetSphereRadius) (.x _returnvalue_2) (.y _returnvalue_2))))))))
  (Class|NiagaraDataInterfaceArrayFunctionLibrary|SetNiagaraArrayVector (Variables|Default|GetNiagara) "User.PointPositions" (Variables|Default|GetPointCloud))
  (Niagara|SetNiagaraVariable(Float) (Variables|Default|GetNiagara) "User.ParticleSize" (Variables|Default|GetParticleSize))
  (Components|Activation|Activate (Variables|Default|GetNiagara) false))

(event EventTick
  (params (DeltaSeconds :type Float%20%28single-precision%29))
  (bind _returnvalue (Game|GetPlayerController 0))
  (bind _returnvalue_2 (Game|GetPlayerCameraManager 0))
  (bind _returnvalue_3 (Transformation|GetActorUpVector))
  (bind _returnvalue_4 (Game|GetPlayerCameraManager 0))
  (bind _rotationsensitivity (Variables|Default|GetRotationSensitivity))
  (bind (_locationx _locationy) (Game|Player|GetMousePosition _returnvalue))
  (bind _returnvalue_5 (Transformation|GetActorForwardVector _returnvalue_4))
  (bind _returnvalue_6 (Math|Vector|DotProduct _returnvalue_3 _returnvalue_5))
  (if (Variables|Default|GetbInspecting)
    (Utilities|FlowControl|Sequence
      (:then_0
        (if (Variables|Default|GetbIsDragging)
          (Variables|Default|SetDeltaX (- _locationx (Variables|Default|GetLastMouseX)))
          (Variables|Default|SetDeltaY (- _locationy (Variables|Default|GetLastMouseY)))
          (Variables|Default|SetLastMouseX _locationx)
          (Variables|Default|SetLastMouseY _locationy)
          (Class|Actor|AddActorWorldRotation (Math|Vector|RotatorfromAxisandAngle (Transformation|GetActorRightVector _returnvalue_2) (* (Variables|Default|GetDeltaY) _rotationsensitivity)))
          (Class|Actor|AddActorWorldRotation (Math|Vector|RotatorfromAxisandAngle (Transformation|GetActorUpVector _returnvalue_2) (* (Variables|Default|GetDeltaX) _rotationsensitivity)))))
      (:then_1
        (Niagara|SetNiagaraVariable(Float) (Variables|Default|GetNiagara) "User.LocomotionStrength" (Math|Float|MapRangeClamped _returnvalue_6 1.0 -0.98 2e+01 0.0))
        (if (<= _returnvalue_6 -0.98)
          (if (Variables|Default|GetbHasSolved)
            (Development|PrintString "Success!")
            (else
              (Variables|Default|SetSuccessTimer (+ (Variables|Default|GetSuccessTimer) (Utilities|Time|GetWorldDeltaSeconds)))
              (if (> (Variables|Default|GetSuccessTimer) (Variables|Default|GetSuccessTimeLength))
                (Variables|Default|SetbHasSolved true))))
          (else
            (Variables|Default|SetSuccessTimer 0.0)
            (Variables|Default|SetbHasSolved false)))))))

(event Input|MouseEvents|LeftMouseButton
  (params (Key :type Key%20Structure :default "None"))
  (bind _returnvalue (Game|GetPlayerController 0))
  (bind (_locationx _locationy) (Game|Player|GetMousePosition _returnvalue))
  (:Pressed
    (if (Variables|Default|GetbInspecting)
      (Variables|Default|SetbIsDragging true)
      (Variables|Default|SetLastMouseX _locationx)
      (Variables|Default|SetLastMouseY _locationy)))
  (:Released
    (Variables|Default|SetbIsDragging false)))

(fn ConstructionScript)

(fn SetInputMode0
  (params (bLockInput :type Boolean))
  (bind _returnvalue (Game|GetPlayerController 0))
  (Input|SetIgnoreLookInput _returnvalue bLockInput)
  (Input|SetIgnoreMoveInput _returnvalue bLockInput)
  (bind _output_get (Variables|/Script/Engine.PlayerController|SetbShowMouseCursor _returnvalue bLockInput))
  (if _output_get
    (Input|SetInputModeGameandUI _returnvalue 0 "DoNotLock" false false)
    (else
      (Input|SetInputModeGameOnly _returnvalue false))))

(fn GetIsInspecting
  (return (Variables|Default|GetbInspecting)))