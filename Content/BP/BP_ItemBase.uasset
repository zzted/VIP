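; Base item Blueprint that the player can inspect, flying it up to the first-person camera and back to where it started.
; OnInteract toggles inspection, playing or reversing a Timeline that lerps location and rotation between the transform saved at BeginPlay and a camera-facing pose.
; SetInputMode locks look and move input and shows the cursor while inspecting, and the highlight is cleared when inspection starts.
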(event `self.ReceiveBeginPlay`
  (set `self.OriginalTransform` (`self.K2_GetActorLocation`))
  (set `self.OriginalRotation` (`self.K2_GetActorRotation`))
  (bind _asbp_first_person_character (cast `/Game/FirstPerson/Blueprints/BP_FirstPersonCharacter` (`GameplayStatics.GetPlayerPawn` 0)))
  (set `self.Player` _asbp_first_person_character))

(event `/Game/BP/BPI_Interactable.OnInteract`
  (bind _returnvalue (not (`self.bInspecting`)))
  (bind _firstpersoncamera (`/Game/FirstPerson/Blueprints/BP_FirstPersonCharacter.FirstPersonCamera` (`self.Player`)))
  (if (`self.bInspecting`)
    (bind _output_get (set `self.bInspecting` _returnvalue))
    (`self.SetInputMode` _output_get)
    (bind (_direction _alpha) (`Timeline|Timeline` :!via `Reverse` :!label _label)
      (:`Update`
        (`self.K2_SetActorLocation` (`KismetMathLibrary.VLerp` (`self.OriginalTransform`) (+ (`SceneComponent.K2_GetComponentLocation` _firstpersoncamera) (* (`SceneComponent.GetForwardVector` _firstpersoncamera) (`self.CameraDistance`))) _alpha))
        (`self.K2_SetActorRotation` (`KismetMathLibrary.RLerp` (`self.OriginalRotation`) (`self.TargetRotation`) _alpha))))
    (else
      (bind _output_get_2 (set `self.bInspecting` _returnvalue))
      (`self.SetInputMode` _output_get_2)
      (`self.UnHighlight`)
      (set `self.TargetRotation` (`KismetMathLibrary.MakeRotFromZ` (+ (* (`SceneComponent.GetForwardVector` (`/Game/FirstPerson/Blueprints/BP_FirstPersonCharacter.FirstPersonCamera` (`self.Player`))) -1.0) (`self.RotationOffset`))))
      (goto _label))))

(fn `SetInputMode`
  (params (bLockInput :type Boolean))
  (bind _returnvalue (`GameplayStatics.GetPlayerController` 0))
  (`Controller.SetIgnoreLookInput` _returnvalue bLockInput)
  (`Controller.SetIgnoreMoveInput` _returnvalue bLockInput)
  (bind _output_get (set `PlayerController.bShowMouseCursor` bLockInput _returnvalue))
  (if _output_get
    (`WidgetBlueprintLibrary.SetInputMode_GameAndUIEx` _returnvalue null "DoNotLock" false)
    (else
      (`WidgetBlueprintLibrary.SetInputMode_GameOnly` _returnvalue))))

(fn `UserConstructionScript`)